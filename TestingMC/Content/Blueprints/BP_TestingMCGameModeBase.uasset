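; BP_TestingMCGameModeBase is a game mode that manages the main HUD and pause menu along with cursor and input mode.
; On BeginPlay it creates and shows WBP_MainUI, hides the cursor and switches to game-only input.
; OnPause adds a new WBP_Pause with a visible cursor and UI-only input; OnResume removes it and restores game input.
; It changes only UI and input, without pausing game time.
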(event Custom|OnPause
  (bind _returnvalue (Game|GetPlayerController 0))
  ;[1 1 1] Handle Pause menu
  (Variables|/Script/Engine.PlayerController|SetbShowMouseCursor _returnvalue true)
  (bind _returnvalue_2 (UserInterface|CreateWidget "/Game/Widgets/WBP_Pause.WBP_Pause_C"))
  (bind _output_get (Variables|Default|SetPauseUI _returnvalue_2))
  (UserInterface|Viewport|AddtoViewport _returnvalue_2 0)
  (Input|SetInputModeUIOnly _returnvalue _output_get "DoNotLock" false))

(event Custom|OnResume
  (bind _returnvalue (Game|GetPlayerController 0))
  (bind _pauseui (Variables|Default|GetPauseUI))
  ;[1 1 1] Handle resuming the game
  (Utilities|IsValid _pauseui
    (:Is%20Valid
      (Widget|RemovefromParent _pauseui)
      (Variables|/Script/Engine.PlayerController|SetbShowMouseCursor _returnvalue false)
      (Input|SetInputModeGameOnly _returnvalue false))))

(event EventBeginPlay
  (bind _returnvalue (Game|GetPlayerController 0))
  ;[1 1 1] Set UI, mouse cursor and mode
  (bind _returnvalue_2 (UserInterface|CreateWidget "/Game/Widgets/WBP_MainUI.WBP_MainUI_C"))
  (bind _output_get (Variables|Default|SetMainUI _returnvalue_2))
  (UserInterface|Viewport|AddtoViewport _output_get 0)
  (Variables|/Script/Engine.PlayerController|SetbShowMouseCursor _returnvalue false)
  (Input|SetInputModeGameOnly _returnvalue false))

(fn ConstructionScript)